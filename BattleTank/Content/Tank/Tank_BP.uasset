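; Player-drivable tank pawn Blueprint that wires input to its movement, aiming and camera components.
; On BeginPlay it hands the barrel and turret to TankAiming and both tracks to TankMovement.
; Forward and Right axes feed TankMovement as fly-by-wire intents, and the Fire action calls TankAiming.
; Camera look splits azimuth yaw on a Scene component from altitude pitch on the CameraArm.
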(event EventBeginPlay)

(event Collision|EventActorBeginOverlap
  (params (OtherActor :type Actor%20Object%20Reference)))

(event EventTick
  (params (DeltaSeconds :type Float%20%28single-precision%29)))

(event EventBeginPlay
  ;[1 1 1] Setting Refrences
  (Class|TankAimingComponent|Initialse (Variables|Default|GetTankAiming) (Variables|Default|GetBarrel) (Variables|Default|GetTurrent))
  (Class|TankMovementComponent|TrackReferences (Variables|Default|GetTankMovement) (Variables|Default|GetLeftTrack) (Variables|Default|GetRightTrack)))

(event Input|ActionEvents|InputActionFire
  (params (Key :type Key%20Structure))
  ;[1 1 1] Input
  (:Pressed
    (Class|TankAimingComponent|Fire (Variables|Default|GetTankAiming))))

(event Input|AxisEvents|InputAxisAimAzimuth
  (params (AxisValue :type Float%20%28single-precision%29))
  ;[1 1 1] Input
  (Transformation|AddLocalRotation (Variables|Default|GetScene) (Math|Rotator|MakeRotator 0.0 0.0 AxisValue) false false))

(event Input|AxisEvents|InputAxisAimAltitude
  (params (AxisValue :type Float%20%28single-precision%29))
  ;[1 1 1] Input
  (Transformation|AddLocalRotation (Variables|Default|GetCamera_Arm) (Math|Rotator|MakeRotator 0.0 AxisValue 0.0) false false))

(event Input|AxisEvents|InputAxisForward
  (params (AxisValue :type Float%20%28single-precision%29))
  ;[1 1 1] Movement Fly By Wire
  (Class|TankMovementComponent|IntendMoveForward (Variables|Default|GetTankMovement) AxisValue))

(event Input|AxisEvents|InputAxisRight
  (params (AxisValue :type Float%20%28single-precision%29))
  ;[1 1 1] Movement Fly By Wire
  (Class|TankMovementComponent|IntendTurnRight (Variables|Default|GetTankMovement) AxisValue))

(fn ConstructionScript)